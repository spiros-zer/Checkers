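; Player controller for a checkers game that drives the front-end menus and local player profiles.
; On local BeginPlay it adds the UI input context, creates a layered screen layout and pushes the intro menu onto its tagged menu layer.
; GotoMainMenu loads the profile save, using notifications to route to the opening or create-profile menu.
; Submitted names are saved to that slot, and the opening menu follows even after a failure notice.
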(event Custom|PushIntroMenu
  ;[1 1 1] PushIntroMenu
  (Utilities|FlowControl|Sequence
    (:then_0
      ;;[1 0 0] Debug
      (Development|PrintString "BP_PC_Checkers | PushMainMenu: Pushing OpeningMenu to Menu Layer Stack" false true "(R=1.000000,G=0.000000,B=0.000000,A=1.000000)"))
    (:then_1
      (bind _commonactivatablewidget (CallFunction|TryPushWidgettoLayer "(TagName=\"UI.Layers.Menu\")" "/Game/Blueprints/UI/WBP_IntroMenu.WBP_IntroMenu_C"))
      (Utilities|IsValid _commonactivatablewidget
        (:Is%20Not%20Valid
          (Development|PrintString "BP_PC_Checkers | PushMainMenu: Pushing OpeningMenu failed" false true "(R=1.000000,G=0.000000,B=0.000000,A=1.000000)"))))))

(event EventBeginPlay
  ;[1 1 1] OnBeginplay
  (if (Pawn|IsLocalController)
    ;;[1 1 1] Enhanced Input Setup
    (Input|AddMappingContext (PlayerController|LocalPlayerSubsystems|GetEnhancedInputLocalPlayerSubsystem self) "/Game/Blueprints/Input/IMC_UI_GenericActions.IMC_UI_GenericActions" 0 "(bIgnoreAllPressedKeysUntilRelease=True,bForceImmediately=False,bNotifyUserSettings=False)")
    (Variables|Default|SetbShowMouseCursor true)
    ;;[1 1 1] Pushing Screen Layout
    (bind _returnvalue (UserInterface|CreateWidget (Variables|Default|GetScreenLayoutClass) self))
    (Utilities|IsValid _returnvalue
      (:Is%20Valid
        (bind _output_get (Variables|Default|SetScreenLayout _returnvalue))
        (Utilities|FlowControl|Sequence
          (:then_0
            ;;;[1 0 0] Debug
            (Development|PrintString "BP_PC_Checkers: Pushing ScreenLayout to player screen" false true "(R=1.000000,G=0.000000,B=0.000000,A=1.000000)"))
          (:then_1
            (UserInterface|Viewport|AddtoViewport _output_get 0)
            ;;;[1 1 1 1 14] Pushing IntroMenu
            (CallFunction|PushIntroMenu))))
      (:Is%20Not%20Valid
        (Development|PrintString "BP_PC_Checkers: Created ScreenLayout widget is not valid!" true true "(R=1.000000,G=0.000000,B=0.000000,A=1.000000)")))
    (else
      (Development|PrintString "BP_PC_Checkers: Is not local controller" false true "(R=1.000000,G=0.000000,B=0.000000,A=1.000000)"))))

(event EventGotoMainMenu
  ;[0.0356 0.0356 0.0356] GoToMainMenu
  (if (Pawn|IsLocalPlayerController)
    (bind _savegame (CallFunction|LoadLocalSaveGame))
    (Utilities|IsValid _savegame
      (:Is%20Valid
        (bind _asbp_sg_player_profile (Utilities|Casting|CastToBP_SG_PlayerProfile _savegame)
          (:then
            (Variables|Default|SetLocalSaveGame _asbp_sg_player_profile)
            (|ShowNotificationAcknowledgement "Notification" "Local save game found."
              (:OnResult
                (CallFunction|TryPushWidgettoLayer "(TagName=\"UI.Layers.Menu\")" "/Game/Blueprints/UI/WBP_OpeningMenu.WBP_OpeningMenu_C"))))
          (:CastFailed
            (|ShowNotificationAcknowledgement "Error" "Local save game with name `LocalSaveGame` found, but seems to be corrupted. Delete and retry"
              (:OnResult
                (CallFunction|TryPushWidgettoLayer "(TagName=\"UI.Layers.Menu\")" "/Game/Blueprints/UI/WBP_CreateProfile.WBP_CreateProfile_C"))))))
      (:Is%20Not%20Valid
        (bind _action (|ShowNotificationDual "Player profile not found" "" "Create New" "Login") ; No player profile detected. Prompt to create one
          (:OnResult
            (switch Utilities|FlowControl|Switch|SwitchonENotificationAction _action
              (:Affirmative
                (CallFunction|TryPushWidgettoLayer "(TagName=\"UI.Layers.Menu\")" "/Game/Blueprints/UI/WBP_CreateProfile.WBP_CreateProfile_C")))))))
    (else
      ;;[1 0 0] Debug
      (Development|PrintString "BP_PC_Checkers: Is not local controller" false true "(R=1.000000,G=0.000000,B=0.000000,A=1.000000)"))))

(event EventPlayerProfileNameSubmitted
  (params (InPlayerProfileName :type Text))
  (bind _bhascreatedplayerprofile (CallFunction|CreateandSaveProfile InPlayerProfileName))
  (if _bhascreatedplayerprofile
    _
    (else
      (|ShowNotificationAcknowledgement "Error" "Could not create player profile."
        (:OnResult
          _))))
  (CallFunction|TryPushWidgettoLayer "(TagName=\"UI.Layers.Menu\")" "/Game/Blueprints/UI/WBP_OpeningMenu.WBP_OpeningMenu_C"))

(fn ConstructionScript)

(fn CreateandSaveProfile
  (params (InPlayerProfileName :type Text))
  (Utilities|IsValid (Variables|Default|GetLocalSaveGame)
    (:Is%20Valid
      ;[0.01938 0.01938 0.01938] Save new player profile username in local save game
      (bind _bhassavedgame (CallFunction|SaveProfile InPlayerProfileName :!label _label))
      (if _bhassavedgame
        _
        (else
          (return false))))
    (:Is%20Not%20Valid
      ;[0.01938 0.01938 0.01938] Save Game Creation
      (bind _returnvalue (SaveGame|CreateSaveGameObject "/Game/Blueprints/SaveGame/BP_SG_PlayerProfile.BP_SG_PlayerProfile_C"))
      (bind _output_get (Variables|Default|SetLocalSaveGame _returnvalue))
      (Utilities|IsValid _output_get
        (:Is%20Valid
          (goto _label))
        (:Is%20Not%20Valid
          (return false)))))
  (return true))

(fn GetPlayerProfiles
  (bind _localsavegame (Variables|Default|GetLocalSaveGame))
  (Utilities|IsValid _localsavegame
    (:Is%20Valid
      (return (Variables|/Game/Blueprints/SaveGame/BP_SG_PlayerProfile.BP_SG_PlayerProfile_C|GetPlayerProfileUsernames _localsavegame)))
    (:Is%20Not%20Valid
      ;[1 1 1] Debug
      (Development|PrintString "BP_PC_Checkers | GetPlayerProfiles: SaveGamePlayerProfiles was not valid" true true "(R=1.000000,G=0.000000,B=0.000000,A=1.000000)"))))

(fn LoadLocalSaveGame
  (bind _profileslotname (Variables|Default|GetProfileSlotName))
  (bind _returnvalue (SaveGame|DoesSaveGameExist _profileslotname))
  (if _returnvalue
    (bind _returnvalue_2 (SaveGame|LoadGamefromSlot _profileslotname))
    (return _returnvalue_2)
    (else
      (return 0))))

(fn SaveProfile
  (params (InProfileName :type Text))
  (bind _localsavegame (Variables|Default|GetLocalSaveGame))
  (Default|AddPlayerProfile _localsavegame InProfileName)
  (if true
    (bind _returnvalue (SaveGame|SaveGametoSlot _localsavegame (Variables|Default|GetProfileSlotName)))
    (return _returnvalue)))

(fn TryPushWidgettoLayer
  (params (LayerTag :type Gameplay%20Tag%20Structure) (ActivatableWidgetClass :type Common%20Activatable%20Widget%20Class%20Reference))
  (bind _screenlayout (Variables|Default|GetScreenLayout))
  (Utilities|IsValid _screenlayout
    (:Is%20Valid
      (bind _returnvalue (Class|CheckersScreenLayoutBase|PushWidgettoLayer _screenlayout LayerTag ActivatableWidgetClass))
      (Utilities|IsValid _returnvalue
        (:Is%20Valid
          (return _returnvalue))
        (:Is%20Not%20Valid
          ;[1 0 0] Debug
          (Development|PrintString "BP_PC_Checkers | TryPushWidgetToLayer: Failed, returning nullptr." true true "(R=1.000000,G=0.000000,B=0.000000,A=1.000000)")
          (return 0))))
    (:Is%20Not%20Valid
      (Development|PrintString "BP_PC_Checkers | TryPushWidgetToLayer: ScreenLayoutWidget is null, returning nullptr." true true "(R=1.000000,G=0.000000,B=0.000000,A=1.000000)")
      (return 0))))